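; Game mode for the multiplayer lobby, handling player roster changes, team and bot setup, game type and match start.
; Logins, after a short delay, and logouts are reported to BP_MPLobbyGameState, which also receives team, bot and game type updates.
; Kicks look up the player's state by ID in the game state and call KickPlayer on that player's lobby screen controller.
; Match start passes the level name to StartMultiplayerGame.
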(event Custom|Kick%20Player
  (params (PlayerId :type Integer))
  (bind _asbp_mplobby_game_state (Utilities|Casting|CastToBP_MPLobbyGameState (Game|GetGameState)))
  (bind _asbp_mplobby_screen_controller (Utilities|Casting|CastToBP_MPLobbyScreenController (Game|GetPlayerController (Utilities|Array|Get(acopy) (Variables|/Game/Blueprints/GameMode/MultiPlayer/BP_MPLobbyGameState.BP_MPLobbyGameState_C|GetAllPlayerStates _asbp_mplobby_game_state) PlayerId))))
  (Default|KickPlayer _asbp_mplobby_screen_controller))

(event Custom|UpdatePlayerShooterStateTeam
  (params (PlayerId :type Integer) (Team :type ETeam%20Enum :default "BlueTeam"))
  (bind _asbp_mplobby_game_state (Utilities|Casting|CastToBP_MPLobbyGameState (Game|GetGameState)))
  (Default|UpdateShooterPlayerStateTeam _asbp_mplobby_game_state PlayerId Team))

(event Custom|UpdateBotTeam
  (params (BotId :type Integer) (Team :type ETeam%20Enum :default "BlueTeam"))
  (bind _asbp_mplobby_game_state (Utilities|Casting|CastToBP_MPLobbyGameState (Game|GetGameState)))
  (Default|UpdateBotTeam _asbp_mplobby_game_state BotId Team))

(event Custom|AddBot
  (bind _asbp_mplobby_game_state (Utilities|Casting|CastToBP_MPLobbyGameState (Game|GetGameState)))
  (Default|AddBot _asbp_mplobby_game_state))

(event Custom|RemoveBot
  (params (BotId :type Integer))
  (bind _asbp_mplobby_game_state (Utilities|Casting|CastToBP_MPLobbyGameState (Game|GetGameState)))
  (Default|RemoveBot _asbp_mplobby_game_state BotId))

(event Custom|UpdateGameType
  (params (GameType :type EAllianceMode%20Enum :default "FFA"))
  (bind _asbp_mplobby_game_state (Utilities|Casting|CastToBP_MPLobbyGameState (Game|GetGameState)))
  (Default|UpdateGameType _asbp_mplobby_game_state GameType))

(event Custom|StartMultiplayerMatch
  (params (LevelName :type String))
  (Class|MPGeneralGameMode|StartMultiplayerGame LevelName))

(event EventBeginPlay)

(event EventTick
  (params (DeltaSeconds :type Float%20%28single-precision%29)))

(event EventPostLogin
  (params (NewPlayer :type Player%20Controller%20Object%20Reference))
  (Utilities|FlowControl|Delay 0.5)
  (bind _asbp_mplobby_game_state (Utilities|Casting|CastToBP_MPLobbyGameState (Game|GetGameState)))
  (Default|PlayerJoined _asbp_mplobby_game_state (Variables|/Script/Engine.Controller|GetPlayerState NewPlayer)))

(event EventOnLogout
  (params (ExitingController :type Controller%20Object%20Reference))
  (bind _asplayer_controller (Utilities|Casting|CastToPlayerController ExitingController))
  (bind _asbp_mplobby_game_state (Utilities|Casting|CastToBP_MPLobbyGameState (Game|GetGameState)))
  (Default|PlayerLeft _asbp_mplobby_game_state (Variables|/Script/Engine.Controller|GetPlayerState _asplayer_controller)))

(fn ConstructionScript)